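; BP_DecoratorVolume is an unfinished decorator volume prototype, with empty events and construction script.
; GenerateRandomPointInCircle builds square-root-distributed points from a seeded stream, reusing one random value for radius and angle, while SetNewRandomSeed resets the seed to zero.
; Disconnected, never-run graphs sketch the intended use: scaling a debug cylinder, line-tracing vertically through each point, adding instanced cube meshes and printing Palette density.
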(event EventBeginPlay)

(event Collision|EventActorBeginOverlap
  (params (OtherActor :type Actor%20Object%20Reference)))

(event EventTick
  (params (DeltaSeconds :type Float%20%28single-precision%29)))

(fn ConstructionScript)

(fn Dadadad)

(fn GenerateRandomPointinCircle
  (Utilities|Array|Clear (Variables|DecoratorVolume|Debug|GetPoints))
  (for _index (range 0 (- (Variables|DecoratorVolume|Getsdasdada) 1))
    ;[0 0 0] Save random float for this loop
    (LocalVariables|SetCurrRandFloat%20%28Local%29 (Math|Random|RandomFloatfromStream (Variables|Default|GetRandomSeedStream)))
    (Utilities|FlowControl|Sequence
      (:then_0
        (LocalVariables|SetR%20%28Local%29 (* (.X (Math|Vector2D|BreakVector2D (Variables|Default|GetSize))) (Math|Float|Sqrt (LocalVariables|GetCurrRandFloat%20%28Local%29))))
        ;[0 0 0] Should be 2 x pi x rand() but value of 200 is used cause unreal's default unit is in cm instead of m
        (LocalVariables|SetTheta%20%28Local%29 (* 2e+02 (Math|Trig|GetPI) (LocalVariables|GetCurrRandFloat%20%28Local%29))))
      (:then_1
        (Utilities|Array|Add (LocalVariables|GetPoints%20%28Local%29) (Math|Vector|MakeVector (* (LocalVariables|GetR%20%28Local%29) (Math|Trig|Cos(Radians) (LocalVariables|GetTheta%20%28Local%29))) (* (LocalVariables|GetR%20%28Local%29) (Math|Trig|Sin(Radians) (LocalVariables|GetTheta%20%28Local%29))) 0.0)))))
  (Variables|DecoratorVolume|Debug|SetPoints (LocalVariables|GetPoints%20%28Local%29))
  (return))

(fn SetNewRandomSeed
  (Math|Random|SetRandomStreamSeed (Variables|Default|GetRandomSeedStream) 0))